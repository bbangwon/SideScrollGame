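; One-shot trigger volume that plays the Master_Boss1 level sequence as the first boss cinematic.
; On overlap it disables the box, reveals the BossMesh and PaladinMesh actors, then hides and stops ticking every Character and CharHpBarBP, with player input and gameplay HUD off.
; A timer matched to the sequence duration restores those actors, input and HUD and destroys the trigger, leaving both cinematic meshes visible.
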(event `self.ReceiveBeginPlay`
  (`self.SetActorHiddenInGame` (`self.BossMesh`) true)
  (`self.SetActorHiddenInGame` (`self.PaladinMesh`) true))

(event `self.Box.OnComponentBeginOverlap`
  (params (OverlappedComponent :type "PrimitiveComponent Object Reference") (OtherActor :type "Actor Object Reference") (OtherComp :type "PrimitiveComponent Object Reference") (OtherBodyIndex :type Integer) (bFromSweep :type Boolean) (SweepResult :type "HitResult Structure (by ref)"))
  (`self.SetActorHiddenInGame` (`self.BossMesh`) false)
  (`self.SetActorHiddenInGame` (`self.PaladinMesh`) false)
  (`PrimitiveComponent.SetCollisionEnabled` (`self.Box`) "NoCollision")
  (bind (_outactor _returnvalue) (`LevelSequencePlayer.CreateLevelSequencePlayer` "/Game/Cinematics/Master_Boss1.Master_Boss1"))
  (`MovieSceneSequencePlayer.Play` _returnvalue)
  (`KismetSystemLibrary.K2_SetTimerDelegate` (delegate `OnFinish_Boss1Sequence`) (`TimeManagementBlueprintLibrary.Conv_QualifiedFrameTimeToSeconds` (`MovieSceneSequencePlayer.GetDuration` _returnvalue)))
  (`self.DisableInput` (`GameplayStatics.GetPlayerCharacter` 0) (`GameplayStatics.GetPlayerController` 0))
  (bind _outactors (`GameplayStatics.GetAllActorsOfClass` "/Script/Engine.Actor"))
  (for _array_element _outactors
    (bind _returnvalue_2 (`GameplayStatics.GetObjectClass` _array_element))
    (if (or (`KismetMathLibrary.ClassIsChildOf` _returnvalue_2 "/Script/Engine.Character") (== _returnvalue_2 "/Game/Blueprints/Etc/CharHpBarBP.CharHpBarBP_C"))
      (`self.SetActorHiddenInGame` _array_element true)
      (`self.SetActorTickEnabled` _array_element false)))
  (bind _asside_scroll_game_instance (cast `/Game/Blueprints/SideScrollGameInstance` (`GameplayStatics.GetGameInstance`)))
  (`/Game/Blueprints/SideScrollGameInstance.ShowGamePlayMainWidget` _asside_scroll_game_instance false))

(event `OnFinish_Boss1Sequence`
  (`self.SetActorHiddenInGame` (`self.BossMesh`) false)
  (`self.SetActorHiddenInGame` (`self.PaladinMesh`) false)
  (`self.EnableInput` (`GameplayStatics.GetPlayerCharacter` 0) (`GameplayStatics.GetPlayerController` 0))
  (bind _outactors (`GameplayStatics.GetAllActorsOfClass` "/Script/Engine.Actor"))
  (for _array_element _outactors
    (bind _returnvalue (`GameplayStatics.GetObjectClass` _array_element))
    (if (or (`KismetMathLibrary.ClassIsChildOf` _returnvalue "/Script/Engine.Character") (== _returnvalue "/Game/Blueprints/Etc/CharHpBarBP.CharHpBarBP_C"))
      (`self.SetActorHiddenInGame` _array_element false)
      (`self.SetActorTickEnabled` _array_element true)))
  (`self.K2_DestroyActor`)
  (bind _asside_scroll_game_instance (cast `/Game/Blueprints/SideScrollGameInstance` (`GameplayStatics.GetGameInstance`)))
  (`/Game/Blueprints/SideScrollGameInstance.ShowGamePlayMainWidget` _asside_scroll_game_instance true))

(fn `UserConstructionScript`)