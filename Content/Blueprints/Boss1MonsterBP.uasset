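; Boss 1 monster character, a goblin melee enemy that chases and slashes the player's Paladin hero along the Y axis only.
; Tick measures player distance and drives a state machine from combat idle to follow to attack, returning to ready idle when the player dies.
; Attack-end events repeat or break off slashes, while collision-window events toggle a damage capsule.
; Taking damage briefly swaps the material, and zero HP plays death and disables collision.
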(event `self.ReceiveTick`
  (params (DeltaSeconds :type "Float (single-precision)"))
  (bind _distanceplayercharacter (`self.DistancePlayerCharacter`))
  (`self.SaveDistanceAndDirection`)
  (if (`self.IsDeathPlayerChar`)
    (set `self.CurrentState` "NewEnumerator3"))
  (switch `/Game/Enums/MonsterState` (`self.CurrentState`)
    (:`NewEnumerator0`
      (if (<= _distanceplayercharacter 500.0)
        (set `self.CurrentState` "NewEnumerator1")))
    (:`NewEnumerator1`
      (if (<= _distanceplayercharacter 160.0)
        (set `self.CurrentState` "NewEnumerator2")
        (`self.PlayAnimMontage` "/Game/Mesh/Goblin/AnimMontage/goblin_slash_Montage.goblin_slash_Montage")
        (set `self.IsAttacking` true)
        (else
          (`self.AddMovementInput` (`self.DirectionToPlayerCharacter`)))))
    (:`NewEnumerator2`
      (if (`self.IsAttacking`)
        _
        (elif (> _distanceplayercharacter 180.0)
          (set `self.CurrentState` "NewEnumerator1"))))))

(event `SaveDistanceAndDirection`
  (bind _returnvalue (`GameplayStatics.GetPlayerCharacter` 0))
  (bind _returnvalue_2 (`KismetMathLibrary.MakeVector` 0.0 (.y (- (`self.K2_GetActorLocation` _returnvalue) (`self.K2_GetActorLocation`)))))
  (bind _aspaladin_hero_bp (cast `/Game/Blueprints/PaladinHeroBP` _returnvalue))
  (set `self.IsDeathPlayerChar` (`/Game/Blueprints/PaladinHeroBP.IsDeath` _aspaladin_hero_bp))
  (set `self.DistancePlayerCharacter` (`KismetMathLibrary.VSize` _returnvalue_2))
  (set `self.DirectionToPlayerCharacter` (`KismetMathLibrary.Normal` _returnvalue_2)))

(event `OnAnimEnd_Attack`
  (set `self.IsAttacking` false)
  (if (`self.IsDeathPlayerChar`)
    (set `self.CurrentState` "NewEnumerator3")
    (elif (> (`self.DistancePlayerCharacter`) 180.0)
      (set `self.CurrentState` "NewEnumerator1")
      (else
        (`self.PlayAnimMontage` "/Game/Mesh/Goblin/AnimMontage/goblin_slash_Montage.goblin_slash_Montage")
        (set `self.IsAttacking` true)))))

(event `self.ReceiveAnyDamage`
  (params (Damage :type "Float (single-precision)") (DamageType :type "DamageType Object Reference") (InstigatedBy :type "Controller Object Reference") (DamageCauser :type "Actor Object Reference"))
  (bind _output_get (set `self.Hp` (- (`self.Hp`) Damage)))
  (`self.ChangeDamageColor`)
  (if (<= _output_get 0.0)
    (`self.PlayAnimMontage` "/Game/Mesh/Goblin/AnimMontage/goblin_death_Montage.goblin_death_Montage")
    (set `self.CurrentState` "NewEnumerator4")
    (`PrimitiveComponent.SetCollisionEnabled` (`self.CapsuleComponent`) "NoCollision")
    (`PrimitiveComponent.SetCollisionEnabled` (`self.Capsule`) "NoCollision")))

(event `ChangeDamageColor`
  (bind _mesh (`self.Mesh`))
  (`PrimitiveComponent.SetMaterial` _mesh 1 "/Game/Mesh/Goblin/phong1_Inst.phong1_Inst")
  (`KismetSystemLibrary.Delay` 0.2)
  (`PrimitiveComponent.SetMaterial` _mesh 1 "/Game/Mesh/Goblin/phong1.phong1"))

(event `self.Capsule.OnComponentBeginOverlap`
  (params (OverlappedComponent :type "PrimitiveComponent Object Reference") (OtherActor :type "Actor Object Reference") (OtherComp :type "PrimitiveComponent Object Reference") (OtherBodyIndex :type Integer) (bFromSweep :type Boolean) (SweepResult :type "HitResult Structure (by ref)"))
  (if (!= OtherActor self)
    (`GameplayStatics.ApplyDamage` OtherActor (`self.Atk`) null self)))

(event `OnColStart_Attack`
  (`PrimitiveComponent.SetCollisionEnabled` (`self.Capsule`) "QueryAndPhysics"))

(event `OnColEnd_Attack`
  (`PrimitiveComponent.SetCollisionEnabled` (`self.Capsule`) "NoCollision"))

(fn `UserConstructionScript`)