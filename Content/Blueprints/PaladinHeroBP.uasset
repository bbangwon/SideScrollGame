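; Player-controlled paladin hero with sword-and-shield combat, moving only along world Y (forward/backward input is unwired) and viewed through the Cam view target.
; Attack and jump inputs play montages, with IsAttacking blocking movement, jumps and repeat attacks.
; Attack events toggle a hit capsule that damages "Character"-tagged components on actors lacking the hero's first tag.
; Received damage lowers Hp, briefly swaps the material, and at zero plays death and disables input.
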(event `self.ReceiveBeginPlay`
  (`PlayerController.SetViewTargetWithBlend` (`GameplayStatics.GetPlayerController` 0) (`self.Cam`) 0.0 "VTBlend_Linear" 0.0 false))

(event `InputAxis|LeftRight`
  (params (AxisValue :type "Float (single-precision)"))
  (if (not (`self.isAttacking`))
    (`self.AddMovementInput` (0.0 1.0 0.0) AxisValue)))

(event `InputAxis|FowardBackward`
  (params (AxisValue :type "Float (single-precision)")))

(event `Key|LeftMouseButton`
  (params (Key :type "Key Structure"))
  (:`Pressed`
    (if (not (`self.isAttacking`))
      (set `self.isAttacking` true)
      (`self.PlayAnimMontage` "/Game/Mesh/Paladin2/AnimMontage/sword_and_shield_slash_Montage.sword_and_shield_slash_Montage"))))

(event `OnAnimEnd_Attack`
  (set `self.isAttacking` false))

(event `Key|SpaceBar`
  (params (Key :type "Key Structure"))
  (:`Pressed`
    (if (`NavMovementInterface.IsFalling` (`self.CharacterMovement`))
      _
      (elif (not (`self.isAttacking`))
        (`self.Jump`)
        (`self.PlayAnimMontage` "/Game/Mesh/Paladin2/AnimMontage/sword_and_shield_jump_Montage.sword_and_shield_jump_Montage"))))
  (:`Released`
    (`self.StopJumping`)))

(event `self.OnLanded`
  (params (Hit :type "HitResult Structure (by ref)"))
  (`self.StopAnimMontage` "/Game/Mesh/Paladin2/AnimMontage/sword_and_shield_jump_Montage.sword_and_shield_jump_Montage"))

(event `self.Capsule.OnComponentBeginOverlap`
  (params (OverlappedComponent :type "PrimitiveComponent Object Reference") (OtherActor :type "Actor Object Reference") (OtherComp :type "PrimitiveComponent Object Reference") (OtherBodyIndex :type Integer) (bFromSweep :type Boolean) (SweepResult :type "HitResult Structure (by ref)"))
  (if (!= OtherActor self)
    (if (not (`self.ActorHasTag` OtherActor (`|GetArrayItem` (`self.Tags`))))
      (if (`ActorComponent.ComponentHasTag` OtherComp "Character")
        (`GameplayStatics.ApplyDamage` OtherActor (`self.Atk`) null self)))))

(event `OnCollStart_Attack`
  (`PrimitiveComponent.SetCollisionEnabled` (`self.Capsule`) "QueryAndPhysics"))

(event `OnCollEnd_Attack`
  (`PrimitiveComponent.SetCollisionEnabled` (`self.Capsule`) "NoCollision"))

(event `self.ReceiveAnyDamage`
  (params (Damage :type "Float (single-precision)") (DamageType :type "DamageType Object Reference") (InstigatedBy :type "Controller Object Reference") (DamageCauser :type "Actor Object Reference"))
  (bind _output_get (set `self.Hp` (- (`self.Hp`) Damage)))
  (`self.ChangeDamageColor`)
  (if (<= _output_get 0.0)
    (`self.PlayAnimMontage` "/Game/Mesh/Paladin2/AnimMontage/sword_and_shield_death_Montage.sword_and_shield_death_Montage")
    (set `self.IsDeath` true)
    (`self.DisableInput` null)))

(event `ChangeDamageColor`
  (bind _mesh (`self.Mesh`))
  (`PrimitiveComponent.SetMaterial` _mesh 0 "/Game/Mesh/Paladin/Paladin_MAT_Inst.Paladin_MAT_Inst")
  (`KismetSystemLibrary.Delay` 0.2)
  (`PrimitiveComponent.SetMaterial` _mesh 0 "/Game/Mesh/Paladin/Paladin_MAT.Paladin_MAT"))

(fn `UserConstructionScript`)