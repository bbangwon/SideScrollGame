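; DefaultPlayGameMode is the game mode for boss stages, showing a stage-clear screen once the boss reaches a specific state.
; BeginPlay finds the first actor tagged "Boss" and stores it as a Boss1MonsterBP.
; Tick polls the boss state during Play, then switches to StageClear, adds the StageClear widget, shows the mouse cursor and disables player character input.
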(event `self.ReceiveBeginPlay`
  (bind _outactors (`GameplayStatics.GetAllActorsWithTag` "Boss"))
  (bind _asboss_1monster_bp (cast `/Game/Blueprints/Boss1MonsterBP` (`|GetArrayItem` _outactors)))
  (set `self.Boss` _asboss_1monster_bp))

(event `self.ReceiveTick`
  (params (DeltaSeconds :type "Float (single-precision)"))
  (bind _returnvalue (`GameplayStatics.GetPlayerController` 0))
  (switch `/Game/Enums/GamePlayState` (`self.CurrentGamePlayState`)
    (:`NewEnumerator1`
      (if (`|EnumEquality` (`/Game/Blueprints/Boss1MonsterBP.CurrentState` (`self.Boss`)) "NewEnumerator4")
        (set `self.CurrentGamePlayState` "NewEnumerator2")
        (bind _returnvalue_2 (`|CreateWidget` "/Game/Blueprints/Widget/StageClear.StageClear_C" _returnvalue))
        (`UserWidget.AddToViewport` _returnvalue_2 0)
        (set `PlayerController.bShowMouseCursor` true _returnvalue)
        (`self.DisableInput` (`GameplayStatics.GetPlayerCharacter` 0) (`GameplayStatics.GetPlayerController` 0))))))

(fn `UserConstructionScript`)