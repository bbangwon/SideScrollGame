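; Default monster character that tracks the player along the world Y axis and reacts to damage.
; Each tick it stores Y-only distance and normalized direction to player 0, printing the direction; no movement logic uses them here.
; Damage lowers Hp and briefly swaps a mesh material as a hit flash.
; At zero Hp or below it plays the goblin death montage, without destroying the actor.
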(event `self.ReceiveTick`
  (params (DeltaSeconds :type "Float (single-precision)"))
  (bind _returnvalue (`KismetMathLibrary.MakeVector` 0.0 (.y (- (`self.K2_GetActorLocation` (`GameplayStatics.GetPlayerCharacter` 0)) (`self.K2_GetActorLocation`)))))
  (set `self.DistancePlayerCharacter` (`KismetMathLibrary.VSize` _returnvalue))
  (bind _output_get (set `self.DirectionToPlayerCharacter` (`KismetMathLibrary.Normal` _returnvalue)))
  (`KismetSystemLibrary.PrintString` (`KismetStringLibrary.Conv_VectorToString` _output_get)))

(event `self.ReceiveAnyDamage`
  (params (Damage :type "Float (single-precision)") (DamageType :type "DamageType Object Reference") (InstigatedBy :type "Controller Object Reference") (DamageCauser :type "Actor Object Reference"))
  (bind _output_get (set `self.Hp` (- (`self.Hp`) Damage)))
  (`self.ChangeDamageColor`)
  (if (<= _output_get 0.0)
    (`self.PlayAnimMontage` "/Game/Mesh/Goblin/AnimMontage/goblin_death_Montage.goblin_death_Montage")))

(event `ChangeDamageColor`
  (bind _mesh (`self.Mesh`))
  (`PrimitiveComponent.SetMaterial` _mesh 1 "/Game/Mesh/Goblin/phong1_Inst.phong1_Inst")
  (`KismetSystemLibrary.Delay` 0.2)
  (`PrimitiveComponent.SetMaterial` _mesh 1 "/Game/Mesh/Goblin/phong1.phong1"))

(fn `UserConstructionScript`)